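; BP_BlastZone is a stage boundary trigger that respawns characters who leave the play area and cleans up anything else.
; On box overlap, a BP_TestCharacter loses collision, mesh visibility and input, waits briefly, then teleports to a hardcoded stage-center point and is restored.
; Other overlapping actors receive a DestroyItemMessage interface call.
; Respawn invincibility and support for other character types are noted as unimplemented.
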(event OnComponentBeginOverlap(Box)
  (params (OverlappedComponent :type Primitive%20Component%20Object%20Reference) (OtherActor :type Actor%20Object%20Reference) (OtherComp :type Primitive%20Component%20Object%20Reference) (OtherBodyIndex :type Integer) (bFromSweep :type Boolean) (SweepResult :type Hit%20Result%20Structure%20%28by%20ref%29))
  ;[1 1 1] Sends characters from blast zone to center of stage. Need to set invincibility when character has it
  ;;[1 1 1] On Cast failed, try next char (not impl.), if failed again, call item interface destroy
  (bind _asbp_test_character (Utilities|Casting|CastToBP_TestCharacter OtherActor)
    (:then
      (Collision|SetActorEnableCollision _asbp_test_character false)
      (Rendering|SetVisibility (Variables|/Game/RatPackGame/Characters/TestCharacter/BP_TestCharacter.BP_TestCharacter_C|GetTempStaticMesh _asbp_test_character) false true)
      (Input|DisableInput _asbp_test_character (Game|GetPlayerController (Variables|/Script/Engine.Pawn|GetPlayerState _asbp_test_character)))
      (Utilities|FlowControl|Delay 2.0)
      (Transformation|Teleport _asbp_test_character "150.000000,200.000000,1050.000000" "0, 0, 0")
      (Rendering|SetVisibility (Variables|/Game/RatPackGame/Characters/TestCharacter/BP_TestCharacter.BP_TestCharacter_C|GetTempStaticMesh _asbp_test_character) true true)
      (Input|EnableInput _asbp_test_character (Game|GetPlayerController (Variables|/Script/Engine.Pawn|GetPlayerState _asbp_test_character)))
      (Collision|SetActorEnableCollision _asbp_test_character true))
    (:CastFailed
      (Class|BPIItems|DestroyItem(Message) OtherActor))))

(event EventBeginPlay)

(event Collision|EventActorBeginOverlap
  (params (OtherActor :type Actor%20Object%20Reference)))

(event EventTick
  (params (DeltaSeconds :type Float%20%28single-precision%29)))

(fn ConstructionScript)