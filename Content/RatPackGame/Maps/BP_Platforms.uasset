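; BP_Platforms is a one-way platform that characters can jump up through and drop down from.
; Bottom trigger overlaps switch a BP_TestCharacter capsule's response on a custom trace channel to Overlap, then back to Block on exit.
; The Top trigger opens a gate that lets the Fall event set the passed player's capsule to Overlap.
; Drop-through is noted as working only for controller 1.
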(event OnComponentBeginOverlap(Bottom)
  (params (OverlappedComponent :type Primitive%20Component%20Object%20Reference) (OtherActor :type Actor%20Object%20Reference) (OtherComp :type Primitive%20Component%20Object%20Reference) (OtherBodyIndex :type Integer) (bFromSweep :type Boolean) (SweepResult :type Hit%20Result%20Structure%20%28by%20ref%29))
  ;[1 1 1] Jump through Platform
  (bind _asbp_test_character (Utilities|Casting|CastToBP_TestCharacter OtherActor))
  (Collision|SetCollisionResponsetoChannel (Variables|/Script/Engine.Character|GetCapsuleComponent _asbp_test_character) "ECC_GameTraceChannel3" "ECR_Overlap"))

(event OnComponentEndOverlap(Bottom)
  (params (OverlappedComponent :type Primitive%20Component%20Object%20Reference) (OtherActor :type Actor%20Object%20Reference) (OtherComp :type Primitive%20Component%20Object%20Reference) (OtherBodyIndex :type Integer))
  ;[1 1 1] Jump through Platform
  (bind _asbp_test_character (Utilities|Casting|CastToBP_TestCharacter OtherActor))
  (Collision|SetCollisionResponsetoChannel (Variables|/Script/Engine.Character|GetCapsuleComponent _asbp_test_character) "ECC_GameTraceChannel3" "ECR_Block"))

(event OnComponentBeginOverlap(Top)
  (params (OverlappedComponent :type Primitive%20Component%20Object%20Reference) (OtherActor :type Actor%20Object%20Reference) (OtherComp :type Primitive%20Component%20Object%20Reference) (OtherBodyIndex :type Integer) (bFromSweep :type Boolean) (SweepResult :type Hit%20Result%20Structure%20%28by%20ref%29))
  ;[1 1 1] Drop Through Platform (only works for controller 1, need to figure that out
  (Utilities|FlowControl|Gate false) ; enters at Open
)

(event OnComponentEndOverlap(Top)
  (params (OverlappedComponent :type Primitive%20Component%20Object%20Reference) (OtherActor :type Actor%20Object%20Reference) (OtherComp :type Primitive%20Component%20Object%20Reference) (OtherBodyIndex :type Integer))
  ;[1 1 1] Drop Through Platform (only works for controller 1, need to figure that out
  (Utilities|FlowControl|Gate false) ; enters at Close
)

(event Custom|Fall
  (params (PlayerRef :type BP%20Test%20Character%20Object%20Reference))
  ;[1 1 1] Drop Through Platform (only works for controller 1, need to figure that out
  (Utilities|FlowControl|Gate false
    (:Exit
      (Collision|SetCollisionResponsetoChannel (Variables|/Script/Engine.Character|GetCapsuleComponent PlayerRef) "ECC_GameTraceChannel3" "ECR_Overlap"))))

(event EventBeginPlay)

(event Collision|EventActorBeginOverlap
  (params (OtherActor :type Actor%20Object%20Reference)))

(event EventTick
  (params (DeltaSeconds :type Float%20%28single-precision%29)))

(fn ConstructionScript)