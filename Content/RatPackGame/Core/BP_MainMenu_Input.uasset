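; Main menu input Blueprint that turns Enhanced Input actions into selection and confirm calls on a menu UI reference.
; One second after BeginPlay it adds its input mapping context to the controlling player's Enhanced Input subsystem.
; While MenuInputMoveUp is ongoing, it prints a debug string and checks an axis key value to shift player 1's selection vertically.
; MenuInputConfirm confirms the current selection when started.
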(event Input|EnhancedActionEvents|EnhancedInputActionMenuInputMoveUp
  (params (ActionValue :type Vector%202D%20Structure) (ElapsedSeconds :type Float%20%28double-precision%29) (TriggeredSeconds :type Float%20%28double-precision%29) (InputAction :type Input%20Action%20Object%20Reference :default "/Game/RatPackGame/Core/MenuInputMoveUp.MenuInputMoveUp"))
  (bind _returnvalue (Class|Actor|GetInputAxisKeyValue))
  (bind _uiref (Variables|Default|GetUIRef))
  (:Ongoing
    (Development|PrintString "Hello")
    (if (< -0.05 _returnvalue)
      (Default|ChangeSelection _uiref 1 0 -1)
      (elif (> 0.05 _returnvalue)
        (Default|ChangeSelection _uiref 1 0 1)))))

(event Input|EnhancedActionEvents|EnhancedInputActionMenuInputConfirm
  (params (ActionValue :type Boolean) (ElapsedSeconds :type Float%20%28double-precision%29) (TriggeredSeconds :type Float%20%28double-precision%29) (InputAction :type Input%20Action%20Object%20Reference :default "/Game/RatPackGame/Core/MenuInputConfirm.MenuInputConfirm"))
  (:Started
    (Default|ConfirmSelection (Variables|Default|GetUIRef))))

(event EventBeginPlay
  (Utilities|FlowControl|Delay 1.0)
  (bind _asplayer_controller (Utilities|Casting|CastToPlayerController (Pawn|GetController)))
  (Utilities|IsValid (PlayerController|LocalPlayerSubsystems|GetEnhancedInputLocalPlayerSubsystem _asplayer_controller)
    (:Is%20Valid
      (Input|AddMappingContext (PlayerController|LocalPlayerSubsystems|GetEnhancedInputLocalPlayerSubsystem _asplayer_controller) (Variables|Default|GetInputContext) 0 "(bIgnoreAllPressedKeysUntilRelease=True,bForceImmediately=False)"))))

(fn ConstructionScript)