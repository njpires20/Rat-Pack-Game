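; BP_PlayerController is a player controller that owns the debug HUD widget and relays game values to it.
; BeginPlay calls CreateHUD, which creates the debug widget, stores a reference and adds it to the viewport.
; UpdateStocks writes a player's remaining stock count as formatted text, and UpdateSteam sets the Steam progress bar from a value scaled down from 100.
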(event Custom|Create%20HUD
  ;[1 1 1] Call through not Begin play
  (bind _returnvalue (UserInterface|CreateWidget "/Game/RatPackGame/UI/BP_Debug.BP_Debug_C"))
  (bind _output_get (Variables|Default|SetDebug%20HUD%20Ref _returnvalue))
  (UserInterface|Viewport|AddtoViewport _output_get 0))

(event Custom|UpdateStocks
  (params (StockCount :type Integer) (PlayerNum :type Integer))
  (Rendering|Components|TextRender|SetText (Variables|/Game/RatPackGame/UI/BP_Debug.BP_Debug_C|GetStocksRemaining (Variables|Default|GetDebug%20HUD%20Ref)) (Utilities|Text|FormatText "P{Playernum}: {Stocks} stocks remaining!" PlayerNum StockCount)))

(event Custom|UpdateSteam
  (params (NewSteam :type Float%20%28double-precision%29))
  (Progress|SetPercent (Variables|/Game/RatPackGame/UI/BP_Debug.BP_Debug_C|GetSteam (Variables|Default|GetDebug%20HUD%20Ref)) (/ NewSteam 1e+02)))

(event EventBeginPlay
  (CallFunction|CreateHUD))

(event EventTick
  (params (DeltaSeconds :type Float%20%28single-precision%29)))

(fn ConstructionScript)