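; Per-player input handler for the character select screen, relaying menu actions to the character select UI with its player number.
; After a one-second delay on BeginPlay, it adds an Enhanced Input mapping context for its player controller and enables input.
; The move action turns the axis value into up or down selection changes, throttled by a 0.2-second lockout.
; Confirm and cancel actions call the matching UI functions directly.
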(event Custom|DelayReset
  (Utilities|FlowControl|Delay 0.2)
  (Variables|Default|SetInputDelay false))

(event Input|EnhancedActionEvents|EnhancedInputActionMenuInputConfirm
  (params (ActionValue :type Boolean) (ElapsedSeconds :type Float%20%28double-precision%29) (TriggeredSeconds :type Float%20%28double-precision%29) (InputAction :type Input%20Action%20Object%20Reference :default "/Game/RatPackGame/Core/MenuInputConfirm.MenuInputConfirm"))
  (:Started
    (Default|ConfirmSelection (Variables|Default|GetCharSelectUIRef) (Variables|Default|GetPNum))))

(event Input|EnhancedActionEvents|EnhancedInputActionMenuInputMoveUp
  (params (ActionValue :type Vector%202D%20Structure) (ElapsedSeconds :type Float%20%28double-precision%29) (TriggeredSeconds :type Float%20%28double-precision%29) (InputAction :type Input%20Action%20Object%20Reference :default "/Game/RatPackGame/Core/MenuInputMoveUp.MenuInputMoveUp"))
  (bind _returnvalue (Class|Actor|GetInputAxisKeyValue))
  (bind _pnum (Variables|Default|GetPNum))
  (bind _charselectuiref (Variables|Default|GetCharSelectUIRef))
  (:Ongoing
    (if (not (Variables|Default|GetInputDelay))
      (Variables|Default|SetInputDelay true)
      (CallFunction|DelayReset)
      (if (!= _returnvalue 0.0)
        (if (> 0.3 _returnvalue)
          (Default|ChangeSelection _charselectuiref _pnum 1 -1)
          (elif (< -0.3 _returnvalue)
            (Default|ChangeSelection _charselectuiref _pnum -1 -1)))))))

(event Input|EnhancedActionEvents|EnhancedInputActionMenuInputCancel
  (params (ActionValue :type Boolean) (ElapsedSeconds :type Float%20%28double-precision%29) (TriggeredSeconds :type Float%20%28double-precision%29) (InputAction :type Input%20Action%20Object%20Reference :default "/Game/RatPackGame/Core/MenuInputCancel.MenuInputCancel"))
  (:Started
    (Default|CancelChoice (Variables|Default|GetCharSelectUIRef) (Variables|Default|GetPNum))))

(event EventBeginPlay
  (Utilities|FlowControl|Delay 1.0)
  (bind _asplayer_controller (Utilities|Casting|CastToPlayerController (Pawn|GetController)))
  (Utilities|IsValid (PlayerController|LocalPlayerSubsystems|GetEnhancedInputLocalPlayerSubsystem _asplayer_controller)
    (:Is%20Valid
      (Input|AddMappingContext (PlayerController|LocalPlayerSubsystems|GetEnhancedInputLocalPlayerSubsystem _asplayer_controller) (Variables|Default|GetContextToAdd) 0 "(bIgnoreAllPressedKeysUntilRelease=True,bForceImmediately=False)")
      (Input|EnableInput self _asplayer_controller)
      (Development|PrintString (Utilities|GetDisplayName _asplayer_controller)))))

(fn ConstructionScript)