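; BP_IcicleItem is a throwable icicle item that sets its type, model, damage and launch power in the construction script.
; Throw clears the owner's held meshes, then either drops it with gravity or launches it sideways without gravity, carrying an attached BP_Hitbox.
; While thrown, overlapping anything but the thrower destroys item and hitbox.
; A physical hit on anything except BP_TestCharacter ends the thrown state and removes the hitbox.
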(event OnComponentHit(StaticMesh)
  (params (HitComponent :type Primitive%20Component%20Object%20Reference) (OtherActor :type Actor%20Object%20Reference) (OtherComp :type Primitive%20Component%20Object%20Reference) (NormalImpulse :type Vector :default "0, 0, 0") (Hit :type Hit%20Result%20Structure%20%28by%20ref%29))
  ;[1 1 1] Destroy Item when it is thrown and hits something
  (if (!= OtherActor "/Game/RatPackGame/Characters/TestCharacter/BP_TestCharacter.BP_TestCharacter")
    (Variables|Default|SetThrown false)
    (Actor|DestroyActor (stale EventThrow _returnvalue_2))))

(event OnComponentBeginOverlap(StaticMesh)
  (params (OverlappedComponent :type Primitive%20Component%20Object%20Reference) (OtherActor :type Actor%20Object%20Reference) (OtherComp :type Primitive%20Component%20Object%20Reference) (OtherBodyIndex :type Integer) (bFromSweep :type Boolean) (SweepResult :type Hit%20Result%20Structure%20%28by%20ref%29))
  ;[1 1 1] Destroy Item when it is thrown and hits something
  (if (not (== OtherActor (Variables|Default|GetCurrentOwner)))
    (if (Variables|Default|GetThrown)
      (Development|PrintString "collided with something")
      (Actor|DestroyActor (stale EventThrow _returnvalue_2))
      (Actor|DestroyActor)
      (CallFunction|DestroyItem))))

(event EventBeginPlay
  (|CallParentFunction) ; This node is disabled and will not be called.\nDrag off pins to build functionality.
)

(event Collision|EventActorBeginOverlap
  (params (OtherActor :type Actor%20Object%20Reference))
  (|CallParentFunction OtherActor) ; This node is disabled and will not be called.\nDrag off pins to build functionality.
)

(event EventTick
  (params (DeltaSeconds :type Float%20%28single-precision%29))
  (|CallParentFunction DeltaSeconds) ; This node is disabled and will not be called.\nDrag off pins to build functionality.
)

(event EventThrow
  (params (Owner :type BP%20Test%20Character%20Object%20Reference) (LeftRight :type Float%20%28double-precision%29) (UpDown :type Float%20%28double-precision%29))
  (bind _returnvalue (* LeftRight 9e+02))
  (bind _staticmesh (Variables|Default|GetStaticMesh))
  (Variables|Default|SetCurrentOwner Owner)
  (Development|PrintString "Thown Item")
  (bind _asbp_vash (Utilities|Casting|CastToBP_Vash Owner)
    (:then
      (Components|StaticMesh|SetStaticMesh (Variables|/Game/RatPackGame/Characters/Vash/BP_Vash.BP_Vash_C|GetPipeItemVash _asbp_vash) 0)
      (Components|StaticMesh|SetStaticMesh (Variables|/Game/RatPackGame/Characters/Vash/BP_Vash.BP_Vash_C|GetHeldItemVash _asbp_vash) 0)
      (Components|StaticMesh|SetStaticMesh (Variables|/Game/RatPackGame/Characters/Vash/BP_Vash.BP_Vash_C|GetGearItemVash _asbp_vash) 0))
    (:CastFailed
      (Components|StaticMesh|SetStaticMesh (Variables|/Game/RatPackGame/Characters/TestCharacter/BP_TestCharacter.BP_TestCharacter_C|GetHeldItem Owner) 0)))
  (Collision|SetCollisionResponsetoChannel (Variables|Default|GetStaticMesh) "ECC_Pawn" "ECR_Overlap")
  (Variables|Default|SetThrown true)
  (Variables|/Game/RatPackGame/Characters/TestCharacter/BP_TestCharacter.BP_TestCharacter_C|SetHoldingItem Owner false)
  (if (== _returnvalue 0.0)
    (Physics|SetEnableGravity _staticmesh true)
    (else
      (Physics|SetEnableGravity _staticmesh false)))
  (Physics|SetPhysicsLinearVelocity _staticmesh (Math|Vector|MakeVector _returnvalue 0.0 0.0) false "None")
  (if (!= LeftRight 0.0)
    (Transformation|SetWorldRotation (Variables|Default|GetStaticMesh) (Math|Rotator|MakeRotator 9e+01 0.0 (* LeftRight 9e+01)) false false)
    (bind _returnvalue_2 (Game|SpawnActorfromClass "/Game/RatPackGame/Characters/BP_Hitbox.BP_Hitbox_C" (Math|Transform|MakeTransform "0, 0, 0" "0, 0, 0" "1.500000,1.500000,4.000000") "Undefined" Owner 0))
    (Variables|/Game/RatPackGame/Characters/BP_Hitbox.BP_Hitbox_C|SetHitboxInfo _returnvalue_2 (Utilities|Struct|MakeBPS_HitboxInfo (Variables|Default|GetItemDamage) "0.000000,0.000000,0.000000" (Variables|Default|GetItemLaunchPower) 0.5 0 "None" "0.000000,0.000000,0.000000|0.000000,0.000000,-0.000000|1.000000,1.000000,1.000000"))
    (Transformation|AttachComponentToComponent _returnvalue_2 (Variables|Default|GetPickupCollision) "None" "KeepRelative" "KeepRelative" "KeepRelative" true)
    (Variables|/Game/RatPackGame/Characters/TestCharacter/BP_TestCharacter.BP_TestCharacter_C|SetHoldingItem Owner false)))

(fn ConstructionScript
  (|CallParentFunction)
  (Variables|Default|SetItemType "NewEnumerator5")
  (Variables|Default|SetItemModel "/Game/RatPackGame/Meshes/Items/icicleBIG.icicleBIG")
  (Variables|Default|SetItemDamage 2e+01)
  (Variables|Default|SetItemLaunchPower 1e+02))