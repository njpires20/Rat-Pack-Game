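; BP_SteamCloudItem is a test item Blueprint for a steam cloud item that uses the Windbag model.
; It adds no runtime logic of its own, as its event graph holds only disabled placeholder events.
; After calling the parent, its construction script sets the inherited item type, model, damage and launch power, leaving behavior to the parent class.
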(event EventBeginPlay
  (|CallParentFunction) ; This node is disabled and will not be called.\nDrag off pins to build functionality.
)

(event Collision|EventActorBeginOverlap
  (params (OtherActor :type Actor%20Object%20Reference))
  (|CallParentFunction OtherActor) ; This node is disabled and will not be called.\nDrag off pins to build functionality.
)

(event EventTick
  (params (DeltaSeconds :type Float%20%28single-precision%29))
  (|CallParentFunction DeltaSeconds) ; This node is disabled and will not be called.\nDrag off pins to build functionality.
)

(fn ConstructionScript
  (|CallParentFunction)
  (Variables|Default|SetItemType "NewEnumerator4")
  (Variables|Default|SetItemModel "/Game/RatPackGame/Meshes/Items/windbag.windbag")
  ;[1 1 1] prev 50
  (Variables|Default|SetItemDamage 5.0)
  (Variables|Default|SetItemLaunchPower 2.5e+03))