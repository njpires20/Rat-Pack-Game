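; BP_BrassPipeItem is a throwable pipe item that sets zero damage and a launch power in its construction script.
; Throw clears the owner's held-item meshes, with a separate branch for BP_Vash, then launches the pipe by physics velocity with an attached BP_Hitbox carrying those stats.
; While thrown, overlapping anything but the owner destroys pipe and hitbox.
; Hits count bounces, and past the limit the pipe disarms and drops its hitbox.
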(event OnComponentHit(StaticMesh)
  (params (HitComponent :type Primitive%20Component%20Object%20Reference) (OtherActor :type Actor%20Object%20Reference) (OtherComp :type Primitive%20Component%20Object%20Reference) (NormalImpulse :type Vector :default "0, 0, 0") (Hit :type Hit%20Result%20Structure%20%28by%20ref%29))
  ;[1 1 1] Destroy Item when it is thrown and hits something
  (if (!= OtherActor "/Game/RatPackGame/Characters/TestCharacter/BP_TestCharacter.BP_TestCharacter")
    (if (> (Variables|Default|GetItemBounces) 2)
      (Variables|Default|SetThrown false)
      (Actor|DestroyActor (stale EventThrow _returnvalue))
      (else
        (bind _result (Math|Integer|IncrementInt (Variables|Default|GetItemBounces))
          (:%20%20
            (Variables|Default|SetItemBounces _result)))))))

(event OnComponentBeginOverlap(StaticMesh)
  (params (OverlappedComponent :type Primitive%20Component%20Object%20Reference) (OtherActor :type Actor%20Object%20Reference) (OtherComp :type Primitive%20Component%20Object%20Reference) (OtherBodyIndex :type Integer) (bFromSweep :type Boolean) (SweepResult :type Hit%20Result%20Structure%20%28by%20ref%29))
  ;[1 1 1] Destroy Item when it is thrown and hits something
  (if (not (== OtherActor (Variables|Default|GetCurrentOwner)))
    (if (Variables|Default|GetThrown)
      (Development|PrintString "collided with something")
      (Actor|DestroyActor (stale EventThrow _returnvalue))
      (Actor|DestroyActor)
      (CallFunction|DestroyItem))))

(event EventBeginPlay
  (|CallParentFunction) ; This node is disabled and will not be called.\nDrag off pins to build functionality.
)

(event Collision|EventActorBeginOverlap
  (params (OtherActor :type Actor%20Object%20Reference))
  (|CallParentFunction OtherActor) ; This node is disabled and will not be called.\nDrag off pins to build functionality.
)

(event EventTick
  (params (DeltaSeconds :type Float%20%28single-precision%29))
  (|CallParentFunction DeltaSeconds) ; This node is disabled and will not be called.\nDrag off pins to build functionality.
)

(event EventThrow
  (params (Owner :type BP%20Test%20Character%20Object%20Reference) (LeftRight :type Float%20%28double-precision%29) (UpDown :type Float%20%28double-precision%29))
  (Variables|Default|SetCurrentOwner Owner)
  (Development|PrintString "Thown Item")
  (bind _asbp_vash (Utilities|Casting|CastToBP_Vash Owner)
    (:then
      (Components|StaticMesh|SetStaticMesh (Variables|/Game/RatPackGame/Characters/Vash/BP_Vash.BP_Vash_C|GetPipeItemVash _asbp_vash) 0)
      (Components|StaticMesh|SetStaticMesh (Variables|/Game/RatPackGame/Characters/Vash/BP_Vash.BP_Vash_C|GetHeldItemVash _asbp_vash) 0)
      (Components|StaticMesh|SetStaticMesh (Variables|/Game/RatPackGame/Characters/Vash/BP_Vash.BP_Vash_C|GetGearItemVash _asbp_vash) 0))
    (:CastFailed
      (Components|StaticMesh|SetStaticMesh (Variables|/Game/RatPackGame/Characters/TestCharacter/BP_TestCharacter.BP_TestCharacter_C|GetPipeItem Owner) 0)
      (Components|StaticMesh|SetStaticMesh (Variables|/Game/RatPackGame/Characters/TestCharacter/BP_TestCharacter.BP_TestCharacter_C|GetHeldItem Owner) 0)
      (Components|StaticMesh|SetStaticMesh (Variables|/Game/RatPackGame/Characters/TestCharacter/BP_TestCharacter.BP_TestCharacter_C|GetGearItem Owner) 0)))
  (Collision|SetCollisionResponsetoChannel (Variables|Default|GetStaticMesh) "ECC_Pawn" "ECR_Overlap")
  (Variables|Default|SetThrown true)
  (Physics|SetPhysicsLinearVelocity (Variables|Default|GetStaticMesh) (Math|Vector|MakeVector (* LeftRight 1.5e+03) 0.0 (* UpDown 1.5e+03)) false "None")
  (bind _returnvalue (Game|SpawnActorfromClass "/Game/RatPackGame/Characters/BP_Hitbox.BP_Hitbox_C" (Math|Transform|MakeTransform "0, 0, 0" "0, 0, 0" "1.500000,1.500000,3.000000") "Undefined" Owner 0))
  (Collision|SetCollisionResponsetoChannel (Variables|/Game/RatPackGame/Characters/BP_Hitbox.BP_Hitbox_C|GetBox _returnvalue) "ECC_GameTraceChannel1" "ECR_Overlap")
  (Variables|/Game/RatPackGame/Characters/BP_Hitbox.BP_Hitbox_C|SetHitboxInfo _returnvalue (Utilities|Struct|MakeBPS_HitboxInfo (Variables|Default|GetItemDamage) "0.000000,0.000000,0.000000" (Variables|Default|GetItemLaunchPower) 0.5 0 "None" "0.000000,0.000000,0.000000|0.000000,0.000000,-0.000000|1.000000,1.000000,1.000000"))
  (Transformation|AttachComponentToComponent _returnvalue (Variables|Default|GetPickupCollision) "None" "KeepRelative" "KeepRelative" "KeepRelative" true)
  (Variables|/Game/RatPackGame/Characters/TestCharacter/BP_TestCharacter.BP_TestCharacter_C|SetHoldingItem Owner false))

(fn ConstructionScript
  (|CallParentFunction)
  (Variables|Default|SetItemType "NewEnumerator3")
  (Variables|Default|SetItemModel "/Game/RatPackGame/Meshes/Items/pipe.pipe")
  (Variables|Default|SetItemDamage 0.0)
  (Variables|Default|SetItemLaunchPower 4e+02))