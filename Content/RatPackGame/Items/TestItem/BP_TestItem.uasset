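; BP_TestItem is a pickup item that characters can hold and throw as a damaging physics projectile.
; PickUp shows the model on a holder mesh chosen by item type, with Vash and Octavia cast separately, then destroys the actor.
; Throw clears held meshes, sets velocity from directional input and attaches a spawned BP_Hitbox carrying damage and launch power.
; Hit events count bounces, then disarm the item by removing hitbox and trail.
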(event OnComponentHit(StaticMesh)
  (params (HitComponent :type Primitive%20Component%20Object%20Reference) (OtherActor :type Actor%20Object%20Reference) (OtherComp :type Primitive%20Component%20Object%20Reference) (NormalImpulse :type Vector :default "0, 0, 0") (Hit :type Hit%20Result%20Structure%20%28by%20ref%29))
  ;[1 1 1] Destroy Item when it is thrown and hits something
  (if (Variables|Default|GetThrown)
    (if (!= OtherActor "/Game/RatPackGame/Characters/TestCharacter/BP_TestCharacter.BP_TestCharacter")
      (if (> (Variables|Default|GetItemBounces) 2)
        (Variables|Default|SetThrown false)
        (Actor|DestroyActor (stale EventThrow _returnvalue))
        (Variables|Default|SetItemBounces 0)
        (Components|Activation|Deactivate (Variables|Default|GetTrail))
        (else
          (bind _result (Math|Integer|IncrementInt (Variables|Default|GetItemBounces))
            (:%20%20
              (Variables|Default|SetItemBounces _result))))))))

(event OnComponentBeginOverlap(StaticMesh)
  (params (OverlappedComponent :type Primitive%20Component%20Object%20Reference) (OtherActor :type Actor%20Object%20Reference) (OtherComp :type Primitive%20Component%20Object%20Reference) (OtherBodyIndex :type Integer) (bFromSweep :type Boolean) (SweepResult :type Hit%20Result%20Structure%20%28by%20ref%29))
  ;[1 1 1] Destroy Item when it is thrown and hits something
)

(event EventBeginPlay)

(event Collision|EventActorBeginOverlap
  (params (OtherActor :type Actor%20Object%20Reference)))

(event EventTick
  (params (DeltaSeconds :type Float%20%28single-precision%29)))

(event EventDestroyItem
  (bind _hitbox (Variables|Default|GetHitbox))
  ;[1 1 1] Destroy Item
  (Development|PrintString "Destroying Item")
  (if (Variables|Default|GetThrown)
    (if (Game|IsActorBeingDestroyed _hitbox)
      _
      (else
        (Utilities|FlowControl|Delay 0.1)
        (Actor|DestroyActor _hitbox))))
  (Actor|DestroyActor))

(event EventPickUp
  (params (Owner :type BP%20Test%20Character%20Object%20Reference))
  (bind _itemmodel (Variables|Default|GetItemModel))
  ;[1 1 1] Pick Up
  (Variables|Default|SetCurrentOwner Owner)
  (Development|PrintString "ItemPickup")
  (bind _output_get (Variables|/Game/RatPackGame/Characters/TestCharacter/BP_TestCharacter.BP_TestCharacter_C|SetHeldItemType Owner (Variables|Default|GetItemType)))
  (bind _asbp_vash (Utilities|Casting|CastToBP_Vash Owner)
    (:then
      (switch Utilities|FlowControl|Switch|SwitchonItemEnum _output_get
        (:NewEnumerator0
          (Components|StaticMesh|SetStaticMesh (Variables|/Game/RatPackGame/Characters/Vash/BP_Vash.BP_Vash_C|GetGearItemVash _asbp_vash) _itemmodel :!label _label))
        (:NewEnumerator1
          (Components|StaticMesh|SetStaticMesh (Variables|/Game/RatPackGame/Characters/Vash/BP_Vash.BP_Vash_C|GetHeldItemVash _asbp_vash) _itemmodel :!label _label_2))
        (:NewEnumerator2
          (goto _label))
        (:NewEnumerator3
          (Components|StaticMesh|SetStaticMesh (Variables|/Game/RatPackGame/Characters/Vash/BP_Vash.BP_Vash_C|GetPipeItemVash _asbp_vash) _itemmodel))
        (:NewEnumerator4
          (goto _label_2))
        (:NewEnumerator5
          (Components|StaticMesh|SetStaticMesh (Variables|/Game/RatPackGame/Characters/Vash/BP_Vash.BP_Vash_C|GetIcicleItemVash _asbp_vash) _itemmodel))
        (:NewEnumerator6
          (goto _label_2))))
    (:CastFailed
      (bind _asbp_octavia (Utilities|Casting|CastToBP_Octavia Owner)
        (:then
          (switch Utilities|FlowControl|Switch|SwitchonItemEnum _output_get
            (:NewEnumerator0
              (Components|StaticMesh|SetStaticMesh (Variables|/Game/RatPackGame/Characters/Octavia/BP_Octavia.BP_Octavia_C|GetGearItemOctavia _asbp_octavia) _itemmodel :!label _label_3))
            (:NewEnumerator1
              (Components|StaticMesh|SetStaticMesh (Variables|/Game/RatPackGame/Characters/Octavia/BP_Octavia.BP_Octavia_C|GetHeldItemOctavia _asbp_octavia) _itemmodel :!label _label_4))
            (:NewEnumerator2
              (goto _label_3))
            (:NewEnumerator3
              (Components|StaticMesh|SetStaticMesh (Variables|/Game/RatPackGame/Characters/Octavia/BP_Octavia.BP_Octavia_C|GetPipeItemOctavia _asbp_octavia) _itemmodel))
            (:NewEnumerator4
              (goto _label_4))
            (:NewEnumerator5
              (Components|StaticMesh|SetStaticMesh (Variables|/Game/RatPackGame/Characters/Octavia/BP_Octavia.BP_Octavia_C|GetIcicleItemOctavia _asbp_octavia) _itemmodel))
            (:NewEnumerator6
              (goto _label_4))))
        (:CastFailed
          (switch Utilities|FlowControl|Switch|SwitchonItemEnum _output_get
            (:NewEnumerator0
              (Components|StaticMesh|SetStaticMesh (Variables|/Game/RatPackGame/Characters/TestCharacter/BP_TestCharacter.BP_TestCharacter_C|GetGearItem Owner) _itemmodel :!label _label_5))
            (:NewEnumerator1
              (Components|StaticMesh|SetStaticMesh (Variables|/Game/RatPackGame/Characters/TestCharacter/BP_TestCharacter.BP_TestCharacter_C|GetHeldItem Owner) _itemmodel :!label _label_6))
            (:NewEnumerator2
              (goto _label_5))
            (:NewEnumerator3
              (Components|StaticMesh|SetStaticMesh (Variables|/Game/RatPackGame/Characters/TestCharacter/BP_TestCharacter.BP_TestCharacter_C|GetPipeItem Owner) _itemmodel))
            (:NewEnumerator4
              (goto _label_6))
            (:NewEnumerator5
              (goto _label_6))
            (:NewEnumerator6
              (goto _label_6)))))))
  (Variables|/Game/RatPackGame/Characters/TestCharacter/BP_TestCharacter.BP_TestCharacter_C|SetHoldingItem Owner true)
  (Utilities|FlowControl|DelayUntilNextTick)
  (Development|PrintString "Finished Pickup")
  (Actor|DestroyActor))

(event EventThrow
  (params (Owner :type BP%20Test%20Character%20Object%20Reference) (LeftRight :type Float%20%28double-precision%29) (UpDown :type Float%20%28double-precision%29))
  ;[1 1 1] Throw
  (Components|Activation|Activate (Variables|Default|GetTrail) false)
  (Variables|Default|SetCurrentOwner Owner)
  (Development|PrintString "Thown Item")
  (bind _asbp_vash (Utilities|Casting|CastToBP_Vash Owner)
    (:then
      (Components|StaticMesh|SetStaticMesh (Variables|/Game/RatPackGame/Characters/Vash/BP_Vash.BP_Vash_C|GetPipeItemVash _asbp_vash) 0)
      (Components|StaticMesh|SetStaticMesh (Variables|/Game/RatPackGame/Characters/Vash/BP_Vash.BP_Vash_C|GetHeldItemVash _asbp_vash) 0)
      (Components|StaticMesh|SetStaticMesh (Variables|/Game/RatPackGame/Characters/Vash/BP_Vash.BP_Vash_C|GetGearItemVash _asbp_vash) 0))
    (:CastFailed
      (bind _asbp_octavia (Utilities|Casting|CastToBP_Octavia Owner)
        (:then
          (Components|StaticMesh|SetStaticMesh (Variables|/Game/RatPackGame/Characters/Octavia/BP_Octavia.BP_Octavia_C|GetPipeItemOctavia _asbp_octavia) 0)
          (Components|StaticMesh|SetStaticMesh (Variables|/Game/RatPackGame/Characters/Octavia/BP_Octavia.BP_Octavia_C|GetHeldItemOctavia _asbp_octavia) 0)
          (Components|StaticMesh|SetStaticMesh (Variables|/Game/RatPackGame/Characters/Octavia/BP_Octavia.BP_Octavia_C|GetGearItemOctavia _asbp_octavia) 0))
        (:CastFailed
          (Components|StaticMesh|SetStaticMesh (Variables|/Game/RatPackGame/Characters/TestCharacter/BP_TestCharacter.BP_TestCharacter_C|GetPipeItem Owner) 0)
          (Components|StaticMesh|SetStaticMesh (Variables|/Game/RatPackGame/Characters/TestCharacter/BP_TestCharacter.BP_TestCharacter_C|GetHeldItem Owner) 0)
          (Components|StaticMesh|SetStaticMesh (Variables|/Game/RatPackGame/Characters/TestCharacter/BP_TestCharacter.BP_TestCharacter_C|GetGearItem Owner) 0)))))
  (Collision|SetCollisionResponsetoChannel (Variables|Default|GetStaticMesh) "ECC_Pawn" "ECR_Overlap")
  (Variables|Default|SetThrown true)
  (Physics|SetPhysicsLinearVelocity (Variables|Default|GetStaticMesh) (Math|Vector|MakeVector (* LeftRight 1.5e+03) 0.0 (* UpDown 1.5e+03)) false "None")
  (bind _returnvalue (Game|SpawnActorfromClass "/Game/RatPackGame/Characters/BP_Hitbox.BP_Hitbox_C" (Math|Transform|MakeTransform "0, 0, 0" "0, 0, 0" "1.500000,1.500000,1.500000") "Undefined" self Owner))
  (Variables|Default|SetHitbox _returnvalue)
  (Collision|SetCollisionResponsetoChannel (Variables|/Game/RatPackGame/Characters/BP_Hitbox.BP_Hitbox_C|GetBox _returnvalue) "ECC_GameTraceChannel1" "ECR_Overlap")
  (Variables|/Game/RatPackGame/Characters/BP_Hitbox.BP_Hitbox_C|SetHitboxInfo _returnvalue (Utilities|Struct|MakeBPS_HitboxInfo (Variables|Default|GetItemDamage) "15.000000,0.000000,0.000000" (Variables|Default|GetItemLaunchPower) 0.5 0 "None" "0.000000,0.000000,0.000000|0.000000,0.000000,-0.000000|1.000000,1.000000,1.000000"))
  (Transformation|AttachComponentToComponent _returnvalue (Variables|Default|GetPickupCollision) "None" "KeepRelative" "KeepRelative" "KeepRelative" true)
  (Variables|/Game/RatPackGame/Characters/TestCharacter/BP_TestCharacter.BP_TestCharacter_C|SetHoldingItem Owner false))

(fn ConstructionScript
  (Components|StaticMesh|SetStaticMesh (Variables|Default|GetStaticMesh) (Variables|Default|GetItemModel))
  (Variables|Default|SetItemDamage 1e+01)
  (Variables|Default|SetItemLaunchPower 1.75e+03))