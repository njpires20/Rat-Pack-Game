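; BP_SteamPackItem is a steam pack item that refills the Steam of the character that picks it up.
; On PickUp it adds a fixed amount to the owner's Steam, capped at the maximum, then clears the owner's holding flag and held-item mesh and destroys itself.
; Its construction script calls the parent's and sets the inherited item type.
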(event EventBeginPlay
  (|CallParentFunction) ; This node is disabled and will not be called.\nDrag off pins to build functionality.
)

(event Collision|EventActorBeginOverlap
  (params (OtherActor :type Actor%20Object%20Reference))
  (|CallParentFunction OtherActor) ; This node is disabled and will not be called.\nDrag off pins to build functionality.
)

(event EventTick
  (params (DeltaSeconds :type Float%20%28single-precision%29))
  (|CallParentFunction DeltaSeconds) ; This node is disabled and will not be called.\nDrag off pins to build functionality.
)

(event EventPickUp
  (params (Owner :type BP%20Test%20Character%20Object%20Reference))
  (if (> (+ (Variables|/Game/RatPackGame/Characters/TestCharacter/BP_TestCharacter.BP_TestCharacter_C|GetSteam Owner) 3e+01) 1e+02)
    (Variables|/Game/RatPackGame/Characters/TestCharacter/BP_TestCharacter.BP_TestCharacter_C|SetSteam Owner 1e+02)
    (else
      (Variables|/Game/RatPackGame/Characters/TestCharacter/BP_TestCharacter.BP_TestCharacter_C|SetSteam Owner (+ (Variables|/Game/RatPackGame/Characters/TestCharacter/BP_TestCharacter.BP_TestCharacter_C|GetSteam Owner) 3e+01))))
  (Variables|/Game/RatPackGame/Characters/TestCharacter/BP_TestCharacter.BP_TestCharacter_C|SetHoldingItem Owner false)
  (Components|StaticMesh|SetStaticMesh (Variables|/Game/RatPackGame/Characters/TestCharacter/BP_TestCharacter.BP_TestCharacter_C|GetHeldItem Owner) 0)
  (Actor|DestroyActor))

(fn ConstructionScript
  (|CallParentFunction)
  (Variables|Default|SetItemType "NewEnumerator6"))